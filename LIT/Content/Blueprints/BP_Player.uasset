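; BP_Player is a 2D flipbook-animated Luffy character that runs, jumps and punches, and loses on touching a BP_Enemy.
; Enhanced Input drives movement and flipbook swaps, all blocked during jumps, with landing detected by polling vertical velocity on a delay loop.
; While a punch plays, Tick calls HitCheck to damage other BP_Player actors overlapping the Box every frame.
; Received damage is only printed, while enemy capsule overlap shows UI_LOSE with UI-only input.
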(event OnFinishedPlaying(Sprite)
  (Sprite|SetFlipbook (Variables|Default|GetSprite) "/Game/Assets/FP_LUFFY_idle.FP_LUFFY_idle")
  (CallFunction|RestartAnim)
  (Variables|Default|Setis_attacking false))

(event OnComponentBeginOverlap(CapsuleComponent)
  (params (OverlappedComponent :type Primitive%20Component%20Object%20Reference) (OtherActor :type Actor%20Object%20Reference) (OtherComp :type Primitive%20Component%20Object%20Reference) (OtherBodyIndex :type Integer) (bFromSweep :type Boolean) (SweepResult :type Hit%20Result%20Structure%20%28by%20ref%29))
  (bind _returnvalue (Game|GetPlayerController 0))
  (Utilities|Casting|CastToBP_Enemy OtherActor)
  (bind _returnvalue_2 (UserInterface|CreateWidget "/Game/Blueprints/UI_LOSE.UI_LOSE_C"))
  (UserInterface|Viewport|AddtoViewport _returnvalue_2 0)
  (Input|SetInputModeUIOnly _returnvalue 0 "DoNotLock" false)
  (Variables|/Script/Engine.PlayerController|SetbShowMouseCursor _returnvalue true))

(event Input|EnhancedActionEvents|EnhancedInputActionIA_Movement
  (params (ActionValue :type Float%20%28double-precision%29) (ElapsedSeconds :type Float%20%28double-precision%29) (TriggeredSeconds :type Float%20%28double-precision%29) (InputAction :type Input%20Action%20Object%20Reference :default "/Game/Blueprints/IA_Movement.IA_Movement"))
  (:Triggered
    (if (not (Variables|Default|Getis_jumping))
      (Pawn|Input|AddMovementInput (Transformation|GetActorForwardVector) ActionValue false)
      (Sprite|SetFlipbook (Variables|Default|GetSprite) "/Game/Assets/FP_LUFFY_run.FP_LUFFY_run")
      (if (> ActionValue 0.0)
        (Transformation|SetWorldRotation (Variables|Default|GetSprite) "0.000000,-180.000000,0.000000" false false)
        (else
          (Transformation|SetWorldRotation (Variables|Default|GetSprite) "0, 0, 0" false false)))))
  (:Completed
    (if (not (Variables|Default|Getis_jumping))
      (Sprite|SetFlipbook (Variables|Default|GetSprite) "/Game/Assets/FP_LUFFY_idle.FP_LUFFY_idle"))))

(event Input|EnhancedActionEvents|EnhancedInputActionIA_Jump
  (params (ActionValue :type Boolean) (ElapsedSeconds :type Float%20%28double-precision%29) (TriggeredSeconds :type Float%20%28double-precision%29) (InputAction :type Input%20Action%20Object%20Reference :default "/Game/Blueprints/IA_Jump.IA_Jump"))
  (bind _sprite (Variables|Default|GetSprite))
  (if (not (Variables|Default|Getis_jumping))
    (Variables|Default|Setis_jumping true)
    (Character|Jump)
    (Components|Timeline|SetLooping _sprite false)
    (Sprite|SetFlipbook _sprite "/Game/Assets/FB_LUFFY_jump.FB_LUFFY_jump")
    (Utilities|FlowControl|Delay 0.1)
    (if (== (.Z (Math|Vector|BreakVector (Transformation|GetVelocity))) 0.0) :!label _label
      (Components|Timeline|SetLooping _sprite true)
      (Audio|Components|Audio|Play _sprite)
      (Sprite|SetFlipbook _sprite "/Game/Assets/FP_LUFFY_idle.FP_LUFFY_idle")
      (Variables|Default|Setis_jumping false)
      (else
        (Utilities|FlowControl|Delay 0.1)
        (goto _label)))))

(event Input|EnhancedActionEvents|EnhancedInputActionIA_Attack
  (params (ActionValue :type Boolean) (ElapsedSeconds :type Float%20%28double-precision%29) (TriggeredSeconds :type Float%20%28double-precision%29) (InputAction :type Input%20Action%20Object%20Reference :default "/Game/Blueprints/IA_Attack.IA_Attack"))
  (if (not (Variables|Default|Getis_jumping))
    (Sprite|SetFlipbook (Variables|Default|GetSprite) "/Game/Assets/LUFFY_PUNCH.LUFFY_PUNCH")
    (Components|Timeline|SetLooping (Variables|Default|GetSprite) false)
    (Variables|Default|Setis_attacking true)))

(event EventBeginPlay
  (bind _asbp_pc (Utilities|Casting|CastToBP_PC (Pawn|GetController)))
  (Input|AddMappingContext (PlayerController|LocalPlayerSubsystems|GetEnhancedInputLocalPlayerSubsystem _asbp_pc) "/Game/Blueprints/IMC_Default.IMC_Default" 0 "(bIgnoreAllPressedKeysUntilRelease=True,bForceImmediately=False,bNotifyUserSettings=False)"))

(event EventTick
  (params (DeltaSeconds :type Float%20%28single-precision%29))
  (if (Variables|Default|Getis_attacking)
    (CallFunction|HitCheck)))

(event Game|Damage|EventAnyDamage
  (params (Damage :type Float%20%28single-precision%29) (DamageType :type Damage%20Type%20Object%20Reference) (InstigatedBy :type Controller%20Object%20Reference) (DamageCauser :type Actor%20Object%20Reference))
  (Development|PrintString (Utilities|String|ToString(Float) Damage)))

(fn ConstructionScript)

(fn RestartAnim
  (Components|Timeline|SetLooping (Variables|Default|GetSprite) true)
  (if (not (Audio|Components|Audio|IsPlaying (Variables|Default|GetSprite)))
    (Audio|Components|Audio|Play (Variables|Default|GetSprite))))

(fn HitCheck
  (for _array_element (Collision|GetOverlappingActors (Variables|Default|GetBox) "BP_Player_C" :!class /Script/Engine.PrimitiveComponent)
    (if (!= _array_element self)
      (Game|Damage|ApplyDamage _array_element (Variables|Default|GetBase%20Damage) 0 0))))